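; BP_VoiceCharacter is a test character for keyboard-driven voice capture and playback.
; On BeginPlay it enables input from player controller 0, then E starts capture and Q stops it.
; W calls PlayVoice after a one-second delay, and Z flips a Switch flag that drives SetOnUDP.
; The Blueprint only wires keys to these voice functions, which are defined outside its graphs.
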(event `self.ReceiveBeginPlay`
  (`self.EnableInput` (`GameplayStatics.GetPlayerController` 0)))

(event `Key|E`
  (params (Key :type "Key Structure"))
  (:`Pressed`
    (`self.ToggleCapture` true)))

(event `Key|Q`
  (params (Key :type "Key Structure"))
  (:`Pressed`
    (`self.ToggleCapture` false)))

(event `Key|W`
  (params (Key :type "Key Structure"))
  (:`Pressed`
    (`KismetSystemLibrary.Delay` 1.0)
    (`self.PlayVoice`)))

(event `Key|Z`
  (params (Key :type "Key Structure"))
  (bind _returnvalue (not (`self.Switch`)))
  (:`Pressed`
    (`self.SetOnUDP` _returnvalue)
    (set `self.Switch` _returnvalue)))

(fn `UserConstructionScript`)