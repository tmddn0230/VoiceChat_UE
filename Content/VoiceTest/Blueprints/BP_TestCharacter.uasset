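; Voice-command test character that opens a trunk or front door from spoken keywords.
; G toggles recognition, which streams microphone audio from a capturable sound wave into a speech recognizer set to Korean without translation.
; Recognized segments are matched against English "open" plus "trunk" or "front", and unmatched text is printed on screen.
; Looping timers step control roll values to animate each opening, with only the trunk guarded against reopening.
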(event `Key|G`
  (params (Key :type "Key Structure"))
  (:`Pressed`
    (if (`self.isActive_Recognizer`)
      (`self.StopRecognition`)
      (set `self.isActive_Recognizer` false)
      (`KismetSystemLibrary.PrintString` "Stop Recognition")
      (else
        (`self.Start_Recognition`)
        (set `self.isActive_Recognizer` true)
        (`KismetSystemLibrary.PrintString` "Start Recognition")))))

(event `self.ReceiveBeginPlay`
  (`self.EnableInput` (`GameplayStatics.GetPlayerController` 0))
  (`self.InitializeRecognition`))

(event `OpenTrunk`
  ;[0.5813 0.5086 1] Open Trunk
  (if (not (`self.IsOpenDoor`))
    (set `self.BLCtrlRoll` 0.0)
    (set `self.BRCtrlRoll` 0.0)
    (bind _returnvalue (`KismetSystemLibrary.K2_SetTimerDelegate` (delegate `Looping_Trunk`) 0.02 true))))

(event `OpenFrontDoor`
  ;[0.9534 0.4965 1] Open Front Door
  (set `self.FLCtrlRoll` 0.0)
  (bind _returnvalue (`KismetSystemLibrary.K2_SetTimerDelegate` (delegate `Looping_Front`) 0.02 true)))

(event `Looping_Trunk`
  ;[0.5813 0.5086 1] Open Trunk
  (set `self.BLCtrlRoll` (+ (`self.BLCtrlRoll`) -1.0))
  (set `self.BRCtrlRoll` (+ (`self.BRCtrlRoll`) 1.0))
  (if (and (<= (`self.BLCtrlRoll`) -140.0) (>= (`self.BRCtrlRoll`) 140.0))
    (`KismetSystemLibrary.K2_ClearAndInvalidateTimerHandle` (stale `OpenTrunk` _returnvalue))
    (set `self.IsOpenDoor` true)))

(event `Looping_Front`
  ;[0.9534 0.4965 1] Open Front Door
  (set `self.FLCtrlRoll` (+ (`self.FLCtrlRoll`) -1.0))
  (if (<= (`self.FLCtrlRoll`) -70.0)
    (`KismetSystemLibrary.K2_ClearAndInvalidateTimerHandle` (stale `OpenFrontDoor` _returnvalue))))

(event `InitializeRecognition`
  ;[1 0.9175 0.3312 1 28] InitializeRecognition
  (bind _returnvalue (`CapturableSoundWave.CreateCapturableSoundWave`))
  (set `self.CapturableSoundWave` _returnvalue)
  (bind _returnvalue_2 (`SpeechRecognizer.CreateSpeechRecognizer`))
  (bind _output_get (set `self.SpeechRecognizer` _returnvalue_2))
  (`SpeechRecognizer.SetRecognitionParameters` _output_get (make `SpeechRecognitionParameters` 0 "Ko" false 5000 true false 0 false 0 0.4 2.4 false))
  (`SpeechRecognizer.SetStreamingDefaults` (`self.SpeechRecognizer`))
  ;;[0.3061 0.1599 1] Captured Audio Check and Process Audio Data
  (add `ImportedSoundWave.OnPopulateAudioData` (`self.CapturableSoundWave`) (delegate `OnPropulateAudioData_Event`)))

(event `OnPropulateAudioData_Event`
  (params (PopulatedAudioData :type "Array of Float (single-precision) (by ref)"))
  (bind _capturablesoundwave (`self.CapturableSoundWave`))
  (bind _speechrecognizer (`self.SpeechRecognizer`))
  ;[1 0.9175 0.3312 1 28] InitializeRecognition
  ;;[0.3061 0.1599 1] Captured Audio Check and Process Audio Data
  (if (not (or (`SpeechRecognizer.GetIsStopped` _speechrecognizer) (`SpeechRecognizer.GetIsStopping` _speechrecognizer)))
    (`SpeechRecognizer.ProcessAudioData` (`self.SpeechRecognizer`) PopulatedAudioData (`KismetMathLibrary.Conv_IntToDouble` (`ImportedSoundWave.GetSampleRate` _capturablesoundwave)) (`ImportedSoundWave.GetNumOfChannels` _capturablesoundwave) false)
    ;;[0.7411 0.6637 1] Print Out ErrorMsg
    (add `SpeechRecognizer.OnRecognitionError` (`self.SpeechRecognizer`) (delegate `OnRecognitionError_Event`))
    ;;[1 0.3146 0.5063] Check Result of Recognized String
    (add `SpeechRecognizer.OnRecognizedTextSegment` (`self.SpeechRecognizer`) (delegate `OnRecognizedTextSegment_Event`))
    ;;[0.5558 1 0.5477] Called PrintString When Recognizer Off
    (add `SpeechRecognizer.OnRecognitionStopped` (`self.SpeechRecognizer`) (delegate `OnRecognitionStopped_Event`))))

(event `OnRecognizedTextSegment_Event`
  (params (RecognizedWords :type String))
  ;[1 0.9175 0.3312 1 28] InitializeRecognition
  ;;[1 0.3146 0.5063] Check Result of Recognized String
  (`self.CheckRecognitionString` RecognizedWords))

(event `OnRecognitionStopped_Event`
  ;[1 0.9175 0.3312 1 28] InitializeRecognition
  ;;[0.5558 1 0.5477] Called PrintString When Recognizer Off
  (`KismetSystemLibrary.PrintString` "Speech recognition has stopped. You can now start it again"))

(event `OnRecognitionError_Event`
  (params (ShortErrorMessage :type String) (LongErrorMessage :type String))
  ;[1 0.9175 0.3312 1 28] InitializeRecognition
  ;;[0.7411 0.6637 1] Print Out ErrorMsg
  (`KismetSystemLibrary.PrintString` LongErrorMessage))

(event `Start_Recognition`
  ;[1 0.6459 0.4526 1 28] Control Recognizer
  (if (`SpeechRecognizer.GetIsStopped` (`self.SpeechRecognizer`))
    (`SpeechRecognizer.StartSpeechRecognition` (`self.SpeechRecognizer`) (delegate `OnStartSpeechRecognition_Event`))
    (else
      (`KismetSystemLibrary.PrintString` "Unable to start the recognizer because it hasn't stopped yet."))))

(event `StopRecognition`
  ;[1 0.6459 0.4526 1 28] Control Recognizer
  (if (`SpeechRecognizer.GetIsStopped` (`self.SpeechRecognizer`))
    (`KismetSystemLibrary.PrintString` "Unable to stop the recognizer because it is already stopped.")
    (else
      (`CapturableSoundWave.StopCapture` (`self.CapturableSoundWave`))
      (`SpeechRecognizer.StopSpeechRecognition` (`self.SpeechRecognizer`)))))

(event `OnStartSpeechRecognition_Event`
  (params (bSucceeded :type Boolean))
  ;[1 0.6459 0.4526 1 28] Control Recognizer
  (if bSucceeded
    ;;[0.6962 1 0.5729 1 16] Audio Capture Start : 변경여지 있음. 음성 통신 방식에 따라
    (bind _returnvalue (`CapturableSoundWave.StartCapture` (`self.CapturableSoundWave`) 0))
    (if _returnvalue
      (`KismetSystemLibrary.PrintString` "Speech recognizer started. Please speak into your input device to recognize your speech.")
      (else
        (`KismetSystemLibrary.PrintString` "Unable to capture audio data from the microphone. Please make sure your microphone is connected correctly")))
    (else
      (`KismetSystemLibrary.PrintString` "Unable to start speech recognition."))))

(fn `CheckRecognitionString`
  (params (RecognitionString :type String))
  (locals (RecognizedString :type String))
  (set `local.RecognizedString` RecognitionString)
  (if (`KismetStringLibrary.Contains` (`local.RecognizedString`) "open")
    (if (`KismetStringLibrary.Contains` (`local.RecognizedString`) "trunk")
      (`self.OpenTrunk`)
      (elif (`KismetStringLibrary.Contains` (`local.RecognizedString`) "front")
        (`self.OpenFrontDoor`)
        (else
          (`KismetSystemLibrary.PrintString` (`local.RecognizedString`) true true (struct :`G` 1.0 :`B` 0.003758 :`A` 1.0) 3.0 :!label _label))))
    (else
      (goto _label))))

(fn `UserConstructionScript`)